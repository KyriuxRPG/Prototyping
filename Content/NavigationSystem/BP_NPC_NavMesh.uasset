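; BP_NPC_NavMesh is an NPC pawn that continually follows the player character using AI navigation.
; BeginPlay stores the spawn location and starts MoveNPC, which calls AIMoveTo toward the location of the player's mesh.
; MoveNPC calls itself after a short delay, longer on success than on failure, re-reading the target each time.
; A random reachable-point lookup around the stored origin is left unconnected.
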(event `self.ReceiveBeginPlay`
  (set `self.OriginLocation` (`self.K2_GetActorLocation`))
  (`self.MoveNPC`))

(event `MoveNPC`
  (`|AIMoveTo` self (`SceneComponent.K2_GetComponentLocation` (`Character.Mesh` (`GameplayStatics.GetPlayerCharacter` 0))) null
    (:`OnSuccess`
      (`KismetSystemLibrary.Delay` 0.5))
    (:`OnFail`
      (`KismetSystemLibrary.Delay` 0.2)))
  (`self.MoveNPC`))

(fn `UserConstructionScript`)