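; Monster actor that travels once along the spline of the BP_SplinePath found in the level, starting on BeginPlay.
; The MoveObjectT timeline's play rate is the inverse of TimeToCompleteInSeconds, so that variable controls the trip duration.
; Each update maps the MoveTrack alpha to a distance along the spline and sets the actor's transform, using world-space location but local-space rotation.
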(event `self.ReceiveBeginPlay`
  (bind _returnvalue (`GameplayStatics.GetActorOfClass` "/Game/BP_SplinePath.BP_SplinePath_C"))
  (set `self.REF Spline` _returnvalue)
  (`self.MoveObject`))

(event `MoveObject`
  (bind _spline (`/Game/BP_SplinePath.Spline` (`self.REF Spline`)))
  (`TimelineComponent.SetPlayRate` (`self.Move Object T`) (`KismetMathLibrary.SafeDivide` 1.0 (`self.Time To Complete (In Seconds)`)))
  (bind (_direction _move_track) (`Timeline|Move Object T`)
    (:`Update`
      (bind _returnvalue (`KismetMathLibrary.Lerp` 0.0 (`SplineComponent.GetSplineLength` (`/Game/BP_SplinePath.Spline` (`self.REF Spline`))) _move_track))
      (`self.K2_SetActorTransform` (`KismetMathLibrary.MakeTransform` (`SplineComponent.GetLocationAtDistanceAlongSpline` _spline _returnvalue "World") (`SplineComponent.GetRotationAtDistanceAlongSpline` _spline _returnvalue "Local"))))))

(fn `UserConstructionScript`)